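; BP_DestroyableActor is a platform actor that changes its mesh material by zone and displays a number on a timer widget.
; Separate low, medium and high zone events each pick a random material from their own array for the mesh's first slot.
; An index-change event passes RandomIndex to the Timer_Plarform widget held by its Widget component.
; The graph contains no destruction logic and leaves the construction script empty.
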(event EventOnChangeIndexPlatform
  (bind _astimer_plarform (Utilities|Casting|CastToTimer_Plarform (UserInterface|GetWidget (Variables|Default|GetWidget))))
  (Default|SetRandomNumber _astimer_plarform (Variables|Default|GetRandomIndex)))

(event EventOnChangeLowZone
  (Rendering|Material|SetMaterial (Variables|Character|GetMesh) 0 (.OutItem (Utilities|Array|Random (Variables|Default|GetLowZoneMaterial)))))

(event EventOnChangeMediumZone
  (Rendering|Material|SetMaterial (Variables|Character|GetMesh) 0 (.OutItem (Utilities|Array|Random (Variables|Default|GetMediumZoneMaterial)))))

(event EventOnChangeHighZone
  (Rendering|Material|SetMaterial (Variables|Character|GetMesh) 0 (.OutItem (Utilities|Array|Random (Variables|Default|GetHighZoneMaterial)))))

(fn ConstructionScript)