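; Two-player Squid Game character that handles its own death, goal and score feedback, with CharacterIndex choosing material and HUD placement.
; BeginPlay attaches a mesh to the head socket and shows the random player ID.
; Death enables mesh physics and, like crossing the goal, creates an ID banner; OnSpawnSound, despite its name, spawns a two-second particle effect.
; The popcorn counter polls NumOfHits in an endless 0.1-second Delay loop, re-calling AddToViewport each pass.
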(event EventOnSpawnSound
  (bind _returnvalue (Effects|SpawnEmitteratLocation "/Game/InfinityBladeEffects/Effects/FX_Mobile/combat/P_Charge_Target_Beam_Fire.P_Charge_Target_Beam_Fire" (Transformation|GetActorLocation)))
  (Utilities|FlowControl|Delay 2.0)
  (Components|DestroyComponent _returnvalue))

(event EventOnCrossGoal
  (if (== (Variables|Default|GetCharacterIndex) 0)
    (bind _returnvalue (UserInterface|CreateWidget "/Game/Widgets/Widget_PlayerWin.Widget_PlayerWin_C"))
    (Default|GetPlayerID _returnvalue (Variables|Default|GetRandomCharacterID))
    (UserInterface|Viewport|AddtoViewport _returnvalue 0)
    (else
      (bind _returnvalue_2 (UserInterface|CreateWidget "/Game/Widgets/Widget_PlayerWin.Widget_PlayerWin_C"))
      (Class|UserWidget|SetPositioninViewport _returnvalue_2 "(X=0.000000,Y=42.000000)" true)
      (Default|GetPlayerID _returnvalue_2 (Variables|Default|GetRandomCharacterID))
      (UserInterface|Viewport|AddtoViewport _returnvalue_2 0))))

(event EventBeginPlay
  (Transformation|AttachComponentToComponent (Variables|Default|GetStaticMesh) (Variables|Character|GetMesh) "headSocket" "KeepRelative" "KeepRelative" "KeepRelative" true)
  (Utilities|FlowControl|Delay 0.1)
  (bind _aswidget_random_id (Utilities|Casting|CastToWidget_RandomID (UserInterface|GetWidget (Variables|Default|GetWidget))))
  (Default|SetRandomID _aswidget_random_id (Variables|Default|GetRandomCharacterID))
  (Rendering|Material|SetMaterial (Variables|Character|GetMesh) 0 (select (== (Variables|Default|GetCharacterIndex) 0) (Variables|Default|GetMaterialPlayer2) (Variables|Default|GetMaterialPlayer1))))

(event EventOnWidgetCounter
  (if (== (Variables|Default|GetCharacterIndex) 0)
    (bind _returnvalue (UserInterface|CreateWidget "/Game/Widgets/Widget_Counter.Widget_Counter_C"))
    (Default|GetPopCornCounter _returnvalue (Variables|Default|GetNumOfHits) true :!label _label)
    (UserInterface|Viewport|AddtoViewport _returnvalue 0)
    (Utilities|FlowControl|Delay 0.1)
    (goto _label)
    (else
      (bind _returnvalue_2 (UserInterface|CreateWidget "/Game/Widgets/Widget_Counter.Widget_Counter_C"))
      (Default|GetPopCornCounter _returnvalue_2 (Variables|Default|GetNumOfHits) false :!label _label_2)
      (Class|UserWidget|SetPositioninViewport _returnvalue_2 "(X=800.000000,Y=0.000000)" true)
      (UserInterface|Viewport|AddtoViewport _returnvalue_2 0)
      (Utilities|FlowControl|Delay 0.1)
      (goto _label_2))))

(event EventOnKillCharacter
  (Physics|SetSimulatePhysics (Variables|Character|GetMesh) true)
  (Audio|PlaySoundatLocation "/Game/Media/Sounds/Uh.Uh" "0, 0, 0" "0, 0, 0" 1.0 1.0 0.0 0 0 0 0)
  (if (== (Variables|Default|GetCharacterIndex) 0)
    (bind _returnvalue (UserInterface|CreateWidget "/Game/Widgets/Widget_PlayerDead.Widget_PlayerDead_C"))
    (Default|PlayerLeftID _returnvalue (Variables|Default|GetRandomCharacterID))
    (UserInterface|Viewport|AddtoViewport _returnvalue 0)
    (else
      (bind _returnvalue_2 (UserInterface|CreateWidget "/Game/Widgets/Widget_PlayerDead.Widget_PlayerDead_C"))
      (Class|UserWidget|SetPositioninViewport _returnvalue_2 "(X=0.000000,Y=42.000000)" true)
      (Default|PlayerLeftID _returnvalue_2 (Variables|Default|GetRandomCharacterID))
      (UserInterface|Viewport|AddtoViewport _returnvalue_2 0))))

(fn ConstructionScript)