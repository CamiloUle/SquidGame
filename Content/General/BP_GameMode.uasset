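; BP_GameMode is a game mode Blueprint with helpers for finding player starts and unwired logic for spawning squid-game characters.
; BeginPlay and Tick are empty, so the spawn and CreatePlayer chains never run.
; The disconnected spawn loop matches each BP_SQPlayerStart's Team to a player index, spawns BP_SquidGameCharacter there and sets its CharacterIndex.
; GetPlayerStart and GetSquidGamePlayerStart cache standard and custom start actors respectively.
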(event EventBeginPlay)

(event EventTick
  (params (DeltaSeconds :type Float%20%28single-precision%29)))

(fn ConstructionScript)

(fn GetPlayerStart
  (bind _outactors (Actor|GetAllActorsOfClass "/Script/Engine.PlayerStart"))
  (Variables|Default|SetPlayerStart _outactors))

(fn GetSquidGamePlayerStart
  (bind _outactors (Actor|GetAllActorsOfClass "/Game/Character/BP_SQPlayerStart.BP_SQPlayerStart_C"))
  (Variables|Default|SetSQ_PlayerStart _outactors))