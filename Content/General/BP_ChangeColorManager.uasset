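; BP_ChangeColorManager runs an endless audio cycle from BeginPlay, playing Squid Game sound cues at varying speeds.
; Each round randomly picks the normal, 1.5x or 2x sound variant and plays it in 2D.
; IsPlayingAudio stays true for a hard-coded delay per variant, then turns false for a fixed pause before the next pick.
; Despite the name, it contains no color-change logic, only this timed flag and sound loop.
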(event EventBeginPlay
  (bind _output_get (Variables|Default|SetSoundIndex (Math|Random|RandomIntegerinRange 1 3) :!label _label))
  (if (== _output_get 1)
    (Audio|PlaySound2D "/Game/Media/Sounds/SquidGameSound.SquidGameSound" 1.0 1.0 0.0 0 0)
    (Variables|Default|SetbIsPlayingAudio true)
    (Utilities|FlowControl|Delay 5.4)
    (Variables|Default|SetbIsPlayingAudio false :!label _label_2)
    (Utilities|FlowControl|Delay 3.5)
    (goto _label)
    (elif (== _output_get 2)
      (Audio|PlaySound2D "/Game/Media/Sounds/SquidGameSoundX1_5.SquidGameSoundX1_5" 1.0 1.0 0.0 0 0)
      (Variables|Default|SetbIsPlayingAudio true)
      (Utilities|FlowControl|Delay 3.6)
      (goto _label_2)
      (elif (== _output_get 3)
        (Audio|PlaySound2D "/Game/Media/Sounds/SquidGameSoundX2.SquidGameSoundX2" 1.0 1.0 0.0 0 0)
        (Variables|Default|SetbIsPlayingAudio true)
        (Utilities|FlowControl|Delay 2.7)
        (goto _label_2)))))

(fn ConstructionScript)