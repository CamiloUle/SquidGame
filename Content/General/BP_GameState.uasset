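; BP_GameState is a game state Blueprint that shows the match timer and handles the end of a round.
; BeginPlay creates a Widget_Timer for player 0 and adds it to the viewport.
; The OnEndSceneGame event waits briefly, puts a Widget_EndScene on the player screen, waits again, then reopens the current level to restart the game.
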(event EventBeginPlay
  (bind _returnvalue (UserInterface|CreateWidget "/Game/Widgets/Widget_Timer.Widget_Timer_C" (Game|GetPlayerController 0)))
  (UserInterface|Viewport|AddtoViewport _returnvalue 0))

(event EventTick
  (params (DeltaSeconds :type Float%20%28single-precision%29)))

(event EventOnEndSceneGame
  (Utilities|FlowControl|Delay 3.0)
  (bind _returnvalue (UserInterface|CreateWidget "/Game/Widgets/Widget_EndScene.Widget_EndScene_C" (Game|GetPlayerController 0)))
  (UserInterface|Viewport|AddtoPlayerScreen _returnvalue)
  (Utilities|FlowControl|Delay 4.0)
  (bind _returnvalue_2 (Game|GetCurrentLevelName true))
  (Game|OpenLevel(byName) (Utilities|String|StringToName _returnvalue_2)))

(fn ConstructionScript)